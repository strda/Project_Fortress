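; Base turret whose look changes with its level on two upgrade paths, built from swappable static mesh parts.
; BeginPlay registers two starting meshes, raises path 1 by one and calls Upgrade, which maps each path combination to a mesh set, with none for 0/0 or 3/3.
; AddElementsUpgrade destroys current components, spawns manual-attachment replacements without attaching them, applies a shared material and prints their names.
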(event EventBeginPlay
  (bind _currentmeshes (Variables|Default|GetCurrentMeshes))
  (Utilities|Array|Add _currentmeshes (Variables|Default|GetCylinder_014_Cylinder_025))
  (Utilities|Array|Add _currentmeshes (Variables|Default|GetCylinder_020_Cylinder_031))
  (Math|Integer|IncrementInt (Variables|Default|GetCurrentPath1)
    (:%20%20
      (CallFunction|Upgrade))))

(event Collision|EventActorBeginOverlap
  (params (OtherActor :type Actor%20Object%20Reference)))

(fn ConstructionScript)

(fn AddElementsUpgrade
  (params (NewMesh :type Array%20of%20Static%20Mesh%20Object%20References))
  (bind _currentmeshes (Variables|Default|GetCurrentMeshes))
  (for _array_element _currentmeshes
    (Components|DestroyComponent _array_element))
  (Utilities|Array|Clear _currentmeshes)
  (for _array_element_2 NewMesh
    (bind _returnvalue (AddComponent|AddStaticMeshComponent true))
    (Utilities|Array|Add _currentmeshes _returnvalue)
    (Components|StaticMesh|SetStaticMesh _returnvalue _array_element_2)
    (Rendering|Material|SetMaterial _returnvalue 0 "/Game/StarterContent/Materials/M_AssetPlatform.M_AssetPlatform"))
  (for _array_element_3 _currentmeshes
    (Development|PrintString (Utilities|GetDisplayName _array_element_3)))
  (return _currentmeshes))

(fn Upgrade
  (bind _currentpath1 (Variables|Default|GetCurrentPath1))
  (bind _currentpath2 (Variables|Default|GetCurrentPath2))
  (if (and (== _currentpath1 0) (== _currentpath2 1))
    (CallFunction|AddElementsUpgrade (Utilities|Array|MakeArray "/Game/Models/Turret0_1/Stock01_0.Stock01_0" "/Game/Models/Turret0_1/Barrel01_0.Barrel01_0" "/Game/Models/Turret0_1/Barrel01_1.Barrel01_1"))
    (elif (and (== _currentpath1 0) (== _currentpath2 2))
      (CallFunction|AddElementsUpgrade (Utilities|Array|MakeArray "/Game/Models/Turret0_2/Cylinder_052_Cylinder_077.Cylinder_052_Cylinder_077" "/Game/Models/Turret0_2/Cylinder_053_Cylinder_078.Cylinder_053_Cylinder_078" "/Game/Models/Turret0_2/Cylinder_054_Cylinder_079.Cylinder_054_Cylinder_079" "/Game/Models/Turret0_2/Cylinder_055_Cylinder_080.Cylinder_055_Cylinder_080" "/Game/Models/Turret0_2/Cylinder_056_Cylinder_081.Cylinder_056_Cylinder_081"))
      (elif (and (== _currentpath1 0) (== _currentpath2 3))
        (CallFunction|AddElementsUpgrade (Utilities|Array|MakeArray "/Game/Models/Turret0_3/BigBarrel_Cylinder_101.BigBarrel_Cylinder_101" "/Game/Models/Turret0_3/Cylinder_006_Cylinder_098.Cylinder_006_Cylinder_098"))
        (elif (and (== _currentpath1 1) (== _currentpath2 0))
          (CallFunction|AddElementsUpgrade (Utilities|Array|MakeArray "/Game/Models/Turret1_0/Cylinder_021_Cylinder_032.Cylinder_021_Cylinder_032" "/Game/Models/Turret1_0/Cylinder_022_Cylinder_033.Cylinder_022_Cylinder_033" "/Game/Models/Turret1_0/Cylinder_023_Cylinder_034.Cylinder_023_Cylinder_034" "/Game/Models/Turret1_0/Cylinder_024_Cylinder_035.Cylinder_024_Cylinder_035"))
          (elif (and (== _currentpath1 2) (== _currentpath2 0))
            (CallFunction|AddElementsUpgrade (Utilities|Array|MakeArray "/Game/Models/Turret2_0/Cube_006_Cube_007.Cube_006_Cube_007" "/Game/Models/Turret2_0/Cylinder_026_Cylinder_022.Cylinder_026_Cylinder_022" "/Game/Models/Turret2_0/Cylinder_027_Cylinder_023.Cylinder_027_Cylinder_023" "/Game/Models/Turret2_0/Cylinder_028_Cylinder_036.Cylinder_028_Cylinder_036" "/Game/Models/Turret2_0/Cylinder_029_Cylinder_037.Cylinder_029_Cylinder_037" "/Game/Models/Turret2_0/Cylinder_030_Cylinder_038.Cylinder_030_Cylinder_038" "/Game/Models/Turret2_0/Cylinder_031_Cylinder_039.Cylinder_031_Cylinder_039"))
            (elif (and (== _currentpath1 3) (== _currentpath2 0))
              (CallFunction|AddElementsUpgrade (Utilities|Array|MakeArray "/Game/Models/Turret3_0/Cylinder_057_Cylinder_082.Cylinder_057_Cylinder_082" "/Game/Models/Turret3_0/Cylinder_058_Cylinder_083.Cylinder_058_Cylinder_083" "/Game/Models/Turret3_0/Cylinder_059_Cylinder_084.Cylinder_059_Cylinder_084" "/Game/Models/Turret3_0/Cylinder_060_Cylinder_085.Cylinder_060_Cylinder_085" "/Game/Models/Turret3_0/Cylinder_061_Cylinder_086.Cylinder_061_Cylinder_086" "/Game/Models/Turret3_0/Cylinder_062_Cylinder_087.Cylinder_062_Cylinder_087" "/Game/Models/Turret3_0/Cylinder_065_Cylinder_090.Cylinder_065_Cylinder_090" "/Game/Models/Turret3_0/Cylinder_066_Cylinder_091.Cylinder_066_Cylinder_091" "/Game/Models/Turret3_0/Cylinder_067_Cylinder_092.Cylinder_067_Cylinder_092" "/Game/Models/Turret3_0/Cylinder_068_Cylinder_093.Cylinder_068_Cylinder_093"))
              (elif (and (== _currentpath1 1) (== 1 _currentpath2))
                (CallFunction|AddElementsUpgrade (Utilities|Array|MakeArray "/Game/Models/Turret1_1/Cylinder_032_Cylinder_047.Cylinder_032_Cylinder_047" "/Game/Models/Turret1_1/Cylinder_033_Cylinder_048.Cylinder_033_Cylinder_048" "/Game/Models/Turret1_1/Cylinder_039_Cylinder_049.Cylinder_039_Cylinder_049" "/Game/Models/Turret1_1/Cylinder_042_Cylinder_052.Cylinder_042_Cylinder_052" "/Game/Models/Turret1_1/Cylinder_043_Cylinder_053.Cylinder_043_Cylinder_053" "/Game/Models/Turret1_1/Cylinder_044_Cylinder_054.Cylinder_044_Cylinder_054"))
                (elif (and (== (Variables|Default|GetCurrentPath1) 1) (== 2 (Variables|Default|GetCurrentPath2)))
                  (CallFunction|AddElementsUpgrade (Utilities|Array|MakeArray "/Game/Models/Turret1_2/Cylinder_101_Cylinder_201.Cylinder_101_Cylinder_201" "/Game/Models/Turret1_2/Cylinder_102_Cylinder_202.Cylinder_102_Cylinder_202" "/Game/Models/Turret1_2/Cylinder_103_Cylinder_203.Cylinder_103_Cylinder_203" "/Game/Models/Turret1_2/Cylinder_105_Cylinder_204.Cylinder_105_Cylinder_204" "/Game/Models/Turret1_2/Cylinder_106_Cylinder_205.Cylinder_106_Cylinder_205" "/Game/Models/Turret1_2/Cylinder_108_Cylinder_196.Cylinder_108_Cylinder_196" "/Game/Models/Turret1_2/Cylinder_109_Cylinder_197.Cylinder_109_Cylinder_197" "/Game/Models/Turret1_2/Cylinder_110_Cylinder_198.Cylinder_110_Cylinder_198" "/Game/Models/Turret1_2/Cylinder_111_Cylinder_199.Cylinder_111_Cylinder_199" "/Game/Models/Turret1_2/Cylinder_112_Cylinder_200.Cylinder_112_Cylinder_200"))
                  (elif (and (== (Variables|Default|GetCurrentPath1) 1) (== 3 (Variables|Default|GetCurrentPath2)))
                    (CallFunction|AddElementsUpgrade (Utilities|Array|MakeArray "/Game/Models/Turret1_3/BigBarrel_004_Cylinder_215.BigBarrel_004_Cylinder_215" "/Game/Models/Turret1_3/BigBarrel_005_Cylinder_217.BigBarrel_005_Cylinder_217" "/Game/Models/Turret1_3/Cylinder_107_Cylinder_214.Cylinder_107_Cylinder_214" "/Game/Models/Turret1_3/Cylinder_113_Cylinder_216.Cylinder_113_Cylinder_216"))
                    (elif (and (== (Variables|Default|GetCurrentPath1) 2) (== 1 (Variables|Default|GetCurrentPath2)))
                      (CallFunction|AddElementsUpgrade (Utilities|Array|MakeArray "/Game/Models/Turret2_1/Barrel2_001_Cylinder_017.Barrel2_001_Cylinder_017" "/Game/Models/Turret2_1/Barrel2_002_Cylinder_016.Barrel2_002_Cylinder_016" "/Game/Models/Turret2_1/Barrel2_003_Cylinder_026.Barrel2_003_Cylinder_026" "/Game/Models/Turret2_1/Barrel2_004_Cylinder_028.Barrel2_004_Cylinder_028" "/Game/Models/Turret2_1/Barrel2_005_Cylinder_027.Barrel2_005_Cylinder_027" "/Game/Models/Turret2_1/Barrel2_Cylinder_030.Barrel2_Cylinder_030" "/Game/Models/Turret2_1/Cylinder_009_Cylinder_020.Cylinder_009_Cylinder_020" "/Game/Models/Turret2_1/Cylinder_013_Cylinder_024.Cylinder_013_Cylinder_024" "/Game/Models/Turret2_1/Cylinder_018_Cylinder_029.Cylinder_018_Cylinder_029"))
                      (elif (and (== (Variables|Default|GetCurrentPath1) 2) (== 2 (Variables|Default|GetCurrentPath2)))
                        (CallFunction|AddElementsUpgrade (Utilities|Array|MakeArray "/Game/Models/Turret2_2/Cylinder_001_Cylinder_111.Cylinder_001_Cylinder_111" "/Game/Models/Turret2_2/Cylinder_002_Cylinder_112.Cylinder_002_Cylinder_112" "/Game/Models/Turret2_2/Cylinder_034_Cylinder_113.Cylinder_034_Cylinder_113" "/Game/Models/Turret2_2/Cylinder_035_Cylinder_114.Cylinder_035_Cylinder_114" "/Game/Models/Turret2_2/Cylinder_040_Cylinder_115.Cylinder_040_Cylinder_115" "/Game/Models/Turret2_2/Cylinder_048_Cylinder_116.Cylinder_048_Cylinder_116" "/Game/Models/Turret2_2/Cylinder_049_Cylinder_117.Cylinder_049_Cylinder_117" "/Game/Models/Turret2_2/Cylinder_063_Cylinder_118.Cylinder_063_Cylinder_118" "/Game/Models/Turret2_2/Cylinder_064_Cylinder_119.Cylinder_064_Cylinder_119" "/Game/Models/Turret2_2/Cylinder_069_Cylinder_120.Cylinder_069_Cylinder_120" "/Game/Models/Turret2_2/Cylinder_070_Cylinder_121.Cylinder_070_Cylinder_121" "/Game/Models/Turret2_2/Cylinder_071_Cylinder_122.Cylinder_071_Cylinder_122" "/Game/Models/Turret2_2/Cylinder_072_Cylinder_123.Cylinder_072_Cylinder_123" "/Game/Models/Turret2_2/Cylinder_073_Cylinder_124.Cylinder_073_Cylinder_124" "/Game/Models/Turret2_2/Cylinder_074_Cylinder_125.Cylinder_074_Cylinder_125"))
                        (elif (and (== (Variables|Default|GetCurrentPath1) 2) (== 3 (Variables|Default|GetCurrentPath2)))
                          (CallFunction|AddElementsUpgrade (Utilities|Array|MakeArray "/Game/Models/Turret2_3/BigBarrel_001_Cylinder_143.BigBarrel_001_Cylinder_143" "/Game/Models/Turret2_3/BigBarrel_002_Cylinder_144.BigBarrel_002_Cylinder_144" "/Game/Models/Turret2_3/BigBarrel_003_Cylinder_145.BigBarrel_003_Cylinder_145" "/Game/Models/Turret2_3/Cylinder_075_Cylinder_130.Cylinder_075_Cylinder_130" "/Game/Models/Turret2_3/Cylinder_080_Cylinder_135.Cylinder_080_Cylinder_135" "/Game/Models/Turret2_3/Cylinder_081_Cylinder_136.Cylinder_081_Cylinder_136"))
                          (elif (and (== (Variables|Default|GetCurrentPath1) 3) (== 1 (Variables|Default|GetCurrentPath2)))
                            (CallFunction|AddElementsUpgrade (Utilities|Array|MakeArray "/Game/Models/Turret3_1/Barrel2_006_Cylinder_060.Barrel2_006_Cylinder_060" "/Game/Models/Turret3_1/Barrel2_007_Cylinder_063.Barrel2_007_Cylinder_063" "/Game/Models/Turret3_1/Barrel2_008_Cylinder_062.Barrel2_008_Cylinder_062" "/Game/Models/Turret3_1/Barrel2_009_Cylinder_064.Barrel2_009_Cylinder_064" "/Game/Models/Turret3_1/Barrel2_010_Cylinder_070.Barrel2_010_Cylinder_070" "/Game/Models/Turret3_1/Barrel2_011_Cylinder_069.Barrel2_011_Cylinder_069" "/Game/Models/Turret3_1/Cylinder_008_Cylinder_061.Cylinder_008_Cylinder_061" "/Game/Models/Turret3_1/Cylinder_015_Cylinder_065.Cylinder_015_Cylinder_065" "/Game/Models/Turret3_1/Cylinder_017_Cylinder_067.Cylinder_017_Cylinder_067" "/Game/Models/Turret3_1/Cylinder_019_Cylinder_071.Cylinder_019_Cylinder_071" "/Game/Models/Turret3_1/Cylinder_045_Cylinder_072.Cylinder_045_Cylinder_072" "/Game/Models/Turret3_1/Cylinder_046_Cylinder_073.Cylinder_046_Cylinder_073" "/Game/Models/Turret3_1/Cylinder_047_Cylinder_074.Cylinder_047_Cylinder_074" "/Game/Models/Turret3_1/Cylinder_050_Cylinder_075.Cylinder_050_Cylinder_075" "/Game/Models/Turret3_1/Cylinder_051_Cylinder_076.Cylinder_051_Cylinder_076"))
                            (elif (and (== (Variables|Default|GetCurrentPath1) 3) (== 2 (Variables|Default|GetCurrentPath2)))
                              (CallFunction|AddElementsUpgrade (Utilities|Array|MakeArray "/Game/Models/Turret3_2/Cylinder_003_Cylinder_168.Cylinder_003_Cylinder_168" "/Game/Models/Turret3_2/Cylinder_005_Cylinder_169.Cylinder_005_Cylinder_169" "/Game/Models/Turret3_2/Cylinder_010_Cylinder_170.Cylinder_010_Cylinder_170" "/Game/Models/Turret3_2/Cylinder_025_Cylinder_171.Cylinder_025_Cylinder_171" "/Game/Models/Turret3_2/Cylinder_076_Cylinder_172.Cylinder_076_Cylinder_172" "/Game/Models/Turret3_2/Cylinder_077_Cylinder_173.Cylinder_077_Cylinder_173" "/Game/Models/Turret3_2/Cylinder_078_Cylinder_174.Cylinder_078_Cylinder_174" "/Game/Models/Turret3_2/Cylinder_082_Cylinder_175.Cylinder_082_Cylinder_175" "/Game/Models/Turret3_2/Cylinder_083_Cylinder_163.Cylinder_083_Cylinder_163" "/Game/Models/Turret3_2/Cylinder_085_Cylinder_164.Cylinder_085_Cylinder_164" "/Game/Models/Turret3_2/Cylinder_086_Cylinder_165.Cylinder_086_Cylinder_165" "/Game/Models/Turret3_2/Cylinder_087_Cylinder_166.Cylinder_087_Cylinder_166" "/Game/Models/Turret3_2/Cylinder_088_Cylinder_167.Cylinder_088_Cylinder_167" "/Game/Models/Turret3_2/Cylinder_089_Cylinder_176.Cylinder_089_Cylinder_176" "/Game/Models/Turret3_2/Cylinder_090_Cylinder_177.Cylinder_090_Cylinder_177" "/Game/Models/Turret3_2/Cylinder_091_Cylinder_178.Cylinder_091_Cylinder_178" "/Game/Models/Turret3_2/Cylinder_092_Cylinder_179.Cylinder_092_Cylinder_179" "/Game/Models/Turret3_2/Cylinder_093_Cylinder_180.Cylinder_093_Cylinder_180" "/Game/Models/Turret3_2/Cylinder_094_Cylinder_181.Cylinder_094_Cylinder_181" "/Game/Models/Turret3_2/Cylinder_095_Cylinder_182.Cylinder_095_Cylinder_182" "/Game/Models/Turret3_2/Cylinder_096_Cylinder_183.Cylinder_096_Cylinder_183" "/Game/Models/Turret3_2/Cylinder_100_Cylinder_187.Cylinder_100_Cylinder_187" "/Game/Models/Turret3_2/Cylinder_097_Cylinder_184.Cylinder_097_Cylinder_184" "/Game/Models/Turret3_2/Cylinder_098_Cylinder_185.Cylinder_098_Cylinder_185" "/Game/Models/Turret3_2/Cylinder_099_Cylinder_186.Cylinder_099_Cylinder_186")))))))))))))))))