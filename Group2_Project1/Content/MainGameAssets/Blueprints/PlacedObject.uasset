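; PlacedObject is a placeable wrapper actor that hosts the placed object through a child actor component.
; BeginPlay spawns RailGunMK1_BP as the child, and SetObj swaps it to CurrentObj.
; Tick switches the child to DestroyedObj behind a child-actor comparison and an always-true branch.
; A TurretFunctionality component lookup is left unused, so no turret state drives that swap.
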(event EventTick
  (params (DeltaSeconds :type Float%20%28single-precision%29))
  (Utilities|FlowControl|Sequence
    (:then_0
      (if (!= (Variables|/Script/Engine.ChildActorComponent|GetChildActor (Variables|Default|GetActor)) 0)
        (if true
          (ChildActorComponent|SetChildActorClass (Variables|Default|GetActor) (Variables|Default|GetDestroyedObj)))))))

(event EventBeginPlay
  (ChildActorComponent|SetChildActorClass (Variables|Default|GetActor) "/Game/MainGameAssets/Blueprints/StaticMeshActor/RailGunMK1_BP.RailGunMK1_BP_C"))

(fn ConstructionScript)

(fn SetObj
  (ChildActorComponent|SetChildActorClass (Variables|Default|GetActor) (Variables|Default|GetCurrentObj)))