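; Homing projectile that damages enemies derived from EnemyBase_BP and destroys itself on hit.
; BeginPlay passes ProjectileMovement to the ProjectileFunctionality component and takes its MoveSpeed for both max speed and homing acceleration.
; SetHoming assigns the homing target, and Sphere overlap applies Damage after an enemy class check.
; A Tick check marked "DO NOT HOOK UP" destroys the projectile when it has no homing target.
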(event OnComponentBeginOverlap(Sphere)
  (params (OverlappedComponent :type Primitive%20Component%20Object%20Reference) (OtherActor :type Actor%20Object%20Reference) (OtherComp :type Primitive%20Component%20Object%20Reference) (OtherBodyIndex :type Integer) (bFromSweep :type Boolean) (SweepResult :type Hit%20Result%20Structure%20%28by%20ref%29))
  (if (Utilities|ClassIsChildOf (Utilities|GetClass (.HitActor (Collision|BreakHitResult SweepResult))) "/Game/MainGameAssets/Blueprints/Enemies/EnemyBase_BP.EnemyBase_BP_C")
    (Game|Damage|ApplyDamage OtherActor (Variables|Default|GetDamage) 0 0)
    (Actor|DestroyActor)))

(event Custom|SetHoming
  (params (Target :type Scene%20Component%20Object%20Reference))
  (bind _output_get (Variables|/Script/Engine.ProjectileMovementComponent|SetHomingTargetComponent (Variables|Default|GetProjectileMovement) Target)))

(event EventBeginPlay
  (bind _projectilefunctionality (Variables|Default|GetProjectileFunctionality))
  (Variables|/Game/MainGameAssets/Blueprints/ProjectileFunctionality.ProjectileFunctionality_C|SetProjectileMovement _projectilefunctionality (Variables|Default|GetProjectileMovement))
  (bind _output_get (Variables|/Script/Engine.ProjectileMovementComponent|SetMaxSpeed (Variables|Default|GetProjectileMovement) (Variables|/Game/MainGameAssets/Blueprints/ProjectileFunctionality.ProjectileFunctionality_C|GetMoveSpeed _projectilefunctionality)))
  (Variables|/Script/Engine.ProjectileMovementComponent|SetHomingAccelerationMagnitude (Variables|Default|GetProjectileMovement) _output_get))

(event EventTick
  (params (DeltaSeconds :type Float%20%28single-precision%29))
  ;[1 1 1] DO NOT HOOK UP
  (if (== (stale Custom|SetHoming _output_get) 0)
    (Actor|DestroyActor)))

(fn ConstructionScript)