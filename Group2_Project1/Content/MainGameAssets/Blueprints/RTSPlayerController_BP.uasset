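; RTS player controller that drives the camera, click selection and building placement.
; BeginPlay spawns the build manager, ghost building and HUD; clicks send hit actors to the HUD or, in build mode, hand non-overlapping ghost placements to the manager.
; Tick blends key input with screen-edge scrolling into bounded camera movement, maps wheel zoom to arm length and pitch, and moves the ghost to the cursor using a zoom-adjusted trace distance.
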(event EventBeginPlay
  (Utilities|FlowControl|Sequence
    (:then_0
      ;[1 1 1] Setting Up Camera on start
      (Variables|References|SetCamPawnRef (Game|Player|GetPlayerPawn 0))
      (Input|SetInputModeGameandUI self 0 "LockAlways" false false)
      (bind _askepler_game_mode (Utilities|Casting|CastToKeplerGameMode (Game|GetGameMode)))
      (Variables|References|SetGameModeRef _askepler_game_mode))
    (:then_1
      (bind _returnvalue (Game|SpawnActorfromClass "/Game/MainGameAssets/Blueprints/BuildingSystemBluePrints/BuildManager_BP.BuildManager_BP_C" (Math|Transform|MakeTransform "0, 0, 0") "AlwaysSpawn" 0 0))
      (Variables|References|SetConstructionManagerRef _returnvalue))
    (:then_2
      (bind _returnvalue_2 (Game|SpawnActorfromClass "/Game/MainGameAssets/Blueprints/BuildingSystemBluePrints/GhostBuilding_BP.GhostBuilding_BP_C" (Math|Transform|MakeTransform "0, 0, 0") "AlwaysSpawn" 0 self 0))
      (Variables|References|SetGhostBuildingRef _returnvalue_2))
    (:then_3
      (bind _returnvalue_3 (UserInterface|CreateWidget "/Game/MainGameAssets/UI/HUD.HUD_C" 0 self (Variables|References|GetGhostBuildingRef) 0))
      (UserInterface|Viewport|AddtoViewport _returnvalue_3 0)
      (Variables|References|SetHUD_REF _returnvalue_3))))

(event EventTick
  (params (DeltaSeconds :type Float%20%28single-precision%29))
  (bind _ghostbuildingref (Variables|References|GetGhostBuildingRef))
  (CallFunction|MoveCamera)
  (if (Variables|/Game/MainGameAssets/Blueprints/KeplerGameMode.KeplerGameMode_C|GetBuildModeActive (Variables|References|GetGameModeRef))
    (if (!= _ghostbuildingref 0)
      (bind _mouselocation (CallFunction|SetCursorWorldPosition self (CallFunction|SetSightDistance)))
      (Default|SetCursorPosition _ghostbuildingref _mouselocation))))

(event Input|ActionEvents|InputActionLeft
  (params (Key :type Key%20Structure :default "None"))
  ;[1 1 1] Camera Move Inputs
  (:Pressed
    (Variables|Default|SetCameraMovement (- (Variables|Default|GetCameraMovement) "1.000000,0.000000,0.000000")))
  (:Released
    (Variables|Default|SetCameraMovement (+ (Variables|Default|GetCameraMovement) "1.000000,0.000000,0.000000"))))

(event Input|ActionEvents|InputActionRight
  (params (Key :type Key%20Structure :default "None"))
  ;[1 1 1] Camera Move Inputs
  (:Pressed
    (Variables|Default|SetCameraMovement (+ (Variables|Default|GetCameraMovement) "1.000000,0.000000,0.000000")))
  (:Released
    (Variables|Default|SetCameraMovement (- (Variables|Default|GetCameraMovement) "1.000000,0.000000,0.000000"))))

(event Input|ActionEvents|InputActionUp
  (params (Key :type Key%20Structure :default "None"))
  ;[1 1 1] Camera Move Inputs
  (:Pressed
    (Variables|Default|SetCameraMovement (- (Variables|Default|GetCameraMovement) "0.000000,1.000000,0.000000")))
  (:Released
    (Variables|Default|SetCameraMovement (+ (Variables|Default|GetCameraMovement) "0.000000,1.000000,0.000000"))))

(event Input|ActionEvents|InputActionDown
  (params (Key :type Key%20Structure :default "None"))
  ;[1 1 1] Camera Move Inputs
  (:Pressed
    (Variables|Default|SetCameraMovement (+ (Variables|Default|GetCameraMovement) "0.000000,1.000000,0.000000")))
  (:Released
    (Variables|Default|SetCameraMovement (- (Variables|Default|GetCameraMovement) "0.000000,1.000000,0.000000"))))

(event Input|ActionEvents|InputActionDeselect
  (params (Key :type Key%20Structure :default "None"))
  ;[1 1 1] Mouse Input and Instance Selection
  (:Pressed
    (if (Variables|/Game/MainGameAssets/Blueprints/KeplerGameMode.KeplerGameMode_C|GetBuildModeActive (Variables|References|GetGameModeRef))
      (Default|KillGhost (Variables|References|GetGhostBuildingRef)))))

(event Input|MouseEvents|MouseWheelUp
  (params (Key :type Key%20Structure :default "None"))
  ;[1 1 1] Camera Zooming
  (:Pressed
    (Variables|Default|SetCameraZoom (Math|Float|Clamp(Float) (- (Variables|Default|GetCameraZoom) 0.2)))))

(event Input|MouseEvents|MouseWheelDown
  (params (Key :type Key%20Structure :default "None"))
  ;[1 1 1] Camera Zooming
  (:Pressed
    (Variables|Default|SetCameraZoom (Math|Float|Clamp(Float) (+ (Variables|Default|GetCameraZoom) 0.2)))))

(event Input|MouseEvents|LeftMouseButton
  (params (Key :type Key%20Structure :default "None"))
  (bind _selectableobjectsenum (Variables|Default|GetSelectableObjectsENUM))
  (bind _ghostbuildingref (Variables|References|GetGhostBuildingRef))
  (bind _hitresult (Class|PlayerController|GetHitResultUnderCursorforObjects _selectableobjectsenum true))
  (bind _hitactor (Collision|BreakHitResult _hitresult))
  ;[1 1 1] Mouse Input and Instance Selection
  (:Pressed
    (Utilities|FlowControl|Sequence
      (:then_0
        (if (!= _hitactor 0)
          (Default|CallHUDRequest _hitactor)
          (else
            (Development|PrintText "AHHH"))))
      (:then_1
        (if (and (Variables|/Game/MainGameAssets/Blueprints/KeplerGameMode.KeplerGameMode_C|GetBuildModeActive (Variables|References|GetGameModeRef)) (== (Default|CheckOverlap (Variables|References|GetGhostBuildingRef)) false))
          (bind _constructionstruct (Default|GetConstructionStruct _ghostbuildingref))
          (Default|ConstructBuilding (Variables|References|GetConstructionManagerRef) _constructionstruct)
          (Default|KillGhost _ghostbuildingref))))))

(event Input|KeyboardEvents|R
  (params (Key :type Key%20Structure :default "None"))
  ;[1 1 1] Rotating Buildings
)

(fn ConstructionScript)

(fn MoveCamera
  (bind _returnvalue (Viewport|GetViewportSize))
  (bind _returnvalue_2 (Viewport|GetViewportSize))
  (bind _camerazoom (Variables|Default|GetCameraZoom))
  (bind _campawnref (Variables|References|GetCamPawnRef))
  (bind _returnvalue_3 (Class|WidgetLayoutLibrary|GetMousePositiononViewport))
  (LocalVariables|SetMouse%20X (.x (* _returnvalue_3 (Class|WidgetLayoutLibrary|GetViewportScale))))
  (LocalVariables|SetMouse%20Y (.y (* _returnvalue_3 (Class|WidgetLayoutLibrary|GetViewportScale))))
  (Transformation|SetActorLocationAndRotation _campawnref (Math|Vector|MakeVector (Math|Float|Clamp(Float) (.x (+ (Transformation|GetActorLocation _campawnref) (* (Math|Vector|Normalize (Utilities|Operators|Subtract (Math|Vector|Normalize (Variables|Default|GetCameraMovement)) (Math|Vector|MakeVector (- 1.0 (Math|Float|Clamp(Float) (Math|Float|NormalizetoRange (LocalVariables|GetMouse%20X) 0.0 (* (.x _returnvalue_2) 0.05)))) 0.0 0.0) (Math|Vector|MakeVector (* -1.0 (Math|Float|Clamp(Float) (Math|Float|NormalizetoRange (LocalVariables|GetMouse%20X) (* (.x _returnvalue_2) 0.95) (.x _returnvalue_2)))) 0.0 0.0) (Math|Vector|MakeVector 0.0 (- 1.0 (Math|Float|Clamp(Float) (Math|Float|NormalizetoRange (LocalVariables|GetMouse%20Y) 0.0 (* (.y _returnvalue) 0.05)))) 0.0) (Math|Vector|MakeVector 0.0 (* -1.0 (Math|Float|Clamp(Float) (Math|Float|NormalizetoRange (LocalVariables|GetMouse%20Y) (* (.y _returnvalue) 0.95) (.y _returnvalue)))) 0.0))) (Math|Float|Lerp (Variables|Default|GetMinCamSpeed) (Variables|Default|GetMaxCamSpeed) 0.0)))) -7e+03 7e+03) (Math|Float|Clamp(Float) (.y (+ (Transformation|GetActorLocation _campawnref) (* (Math|Vector|Normalize (Utilities|Operators|Subtract (Math|Vector|Normalize (Variables|Default|GetCameraMovement)) (Math|Vector|MakeVector (- 1.0 (Math|Float|Clamp(Float) (Math|Float|NormalizetoRange (LocalVariables|GetMouse%20X) 0.0 (* (.x _returnvalue_2) 0.05)))) 0.0 0.0) (Math|Vector|MakeVector (* -1.0 (Math|Float|Clamp(Float) (Math|Float|NormalizetoRange (LocalVariables|GetMouse%20X) (* (.x _returnvalue_2) 0.95) (.x _returnvalue_2)))) 0.0 0.0) (Math|Vector|MakeVector 0.0 (- 1.0 (Math|Float|Clamp(Float) (Math|Float|NormalizetoRange (LocalVariables|GetMouse%20Y) 0.0 (* (.y _returnvalue) 0.05)))) 0.0) (Math|Vector|MakeVector 0.0 (* -1.0 (Math|Float|Clamp(Float) (Math|Float|NormalizetoRange (LocalVariables|GetMouse%20Y) (* (.y _returnvalue) 0.95) (.y _returnvalue)))) 0.0))) (Math|Float|Lerp (Variables|Default|GetMinCamSpeed) (Variables|Default|GetMaxCamSpeed) 0.0)))) -7e+03 7e+03) 1.5e+03) (Math|Rotator|MakeRotator 0.0 (Math|Float|Lerp 5.0 0.0 _camerazoom) -9e+01))
  (bind _asrtscamera_pawn_bp (Utilities|Casting|CastToRTSCameraPawn_BP _campawnref))
  (Variables|/Script/Engine.SpringArmComponent|SetTargetArmLength (Variables|/Game/MainGameAssets/Blueprints/RTSCameraPawn_BP.RTSCameraPawn_BP_C|GetSpringArm _asrtscamera_pawn_bp) (Math|Float|Lerp (Variables|Default|GetMinCamZoom) (Variables|Default|GetMaxCamZoom) _camerazoom)))

(fn SetSightDistance
  (bind _asrtscamera_pawn_bp (Utilities|Casting|CastToRTSCameraPawn_BP (Variables|References|GetCamPawnRef)))
  (return (+ (Variables|/Script/Engine.SpringArmComponent|GetTargetArmLength (Variables|/Game/MainGameAssets/Blueprints/RTSCameraPawn_BP.RTSCameraPawn_BP_C|GetSpringArm _asrtscamera_pawn_bp)) (Variables|Default|GetSightDistance))))