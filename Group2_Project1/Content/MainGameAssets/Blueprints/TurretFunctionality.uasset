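; Turret logic that makes a parent actor track and fire at enemies in range.
; Each Tick, a sphere overlap picks the nearest EnemyStandard_BP and yaws the rotating object toward it, setting TargetFound.
; While a target is found, a Delay-gated path spawns projectiles at barrel child components, staggering multiple barrels through a hand-built delayed loop.
; Homing turrets set the target's root component as the projectile's homing target.
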(event EventBeginPlay)

(event EventTick
  (params (DeltaSeconds :type Float%20%28single-precision%29))
  (bind _targetfound (Variables|Default|GetTargetFound))
  (bind _barrels (Variables|Components|GetBarrels))
  (bind _returnvalue (Utilities|Array|Length _barrels))
  (Utilities|FlowControl|Sequence :!label _label
    (:then_0
      (if _targetfound
        (Utilities|FlowControl|Delay (Variables|Default|GetFireDelay))
        (if _targetfound
          (if (> (Utilities|Array|Length _barrels) 1)
            (if (< (Variables|Components|GetForEachLoopWait) _returnvalue) :!label _label_2
              (Utilities|FlowControl|Sequence
                (:then_0
                  (if (Variables|Default|GetTargetFound)
                    (CallFunction|Shoot 0 (Components|GetChildComponent (Utilities|Array|Get(acopy) _barrels (Variables|Components|GetForEachLoopWait)) 0))
                    (Development|PrintString "HIIIII" :!label _label_3)
                    (else
                      (goto _label))))
                (:then_1
                  (Math|Integer|IncrementInt (Variables|Components|GetForEachLoopWait)
                    (:%20%20
                      (Utilities|FlowControl|Delay (/ (/ (Variables|Default|GetFireDelay) _returnvalue) 2.0))
                      (goto _label_2)))))
              (else
                (Variables|Components|SetForEachLoopWait 0)))
            (elif (Variables|Default|GetTargetFound)
              (CallFunction|Shoot 0 (Components|GetChildComponent (Utilities|Array|Get(acopy) _barrels) 0))
              (goto _label_3))))))
    (:then_1
      (CallFunction|RotatetoObject))))

(fn RotatetoObject
  (bind _parent (Variables|Default|GetParent))
  (Variables|Default|SetDistanceToTarget 1e+04)
  (bind (_outactors _returnvalue) (Collision|SphereOverlapActors (Transformation|GetActorLocation _parent) (Variables|Default|GetRange) (Utilities|Array|MakeArray "ObjectTypeQuery3") "/Game/MainGameAssets/Blueprints/Enemies/EnemyStandard_BP.EnemyStandard_BP_C")) ; Enemy class will be put in the actor class filter once it is implemented into the game
  (if _returnvalue
    (for _array_element _outactors
      (if (< (Transformation|GetDistanceTo _parent _array_element) (Variables|Default|GetDistanceToTarget))
        (Variables|Default|SetDistanceToTarget (Transformation|GetDistanceTo _parent _array_element))
        (bind _output_get (Variables|Default|SetTargetActor _array_element))))
    (if (Utilities|IsValid _output_get)
      (Transformation|SetRelativeRotation (Variables|Default|GetObjectRotating) (Math|Interpolation|RInterpTo (Transformation|GetActorRotation _parent) (Math|Rotator|MakeRotator 0.0 0.0 (- (.Yaw (Math|Rotator|BreakRotator (Math|Rotator|FindLookatRotation (Transformation|GetActorLocation _parent) (Transformation|GetActorLocation _output_get)))) 9e+01)) 1.0 (Variables|Default|GetInterpSpeed)) false false)
      (Variables|Default|SetTargetFound true))
    (else
      (Variables|Default|SetTargetFound false))))

(fn Shoot
  (params (Arrow :type Arrow%20Component%20Object%20Reference) (NewParam :type Scene%20Component%20Object%20Reference))
  (bind _objectrotating (Variables|Default|GetObjectRotating))
  (bind _targetactor (Variables|Default|GetTargetActor))
  (bind _relativerotation (Variables|/Script/Engine.SceneComponent|GetRelativeRotation _objectrotating))
  (if (Variables|Default|GetTargetFound)
    (bind _returnvalue (Game|SpawnActorfromClass (Variables|Default|GetProjectileType) (Math|Transform|MakeTransform (.location (Transformation|GetWorldTransform NewParam)) (Math|Rotator|MakeRotator (.roll _relativerotation) (.pitch _relativerotation) (+ (.yaw (Variables|/Script/Engine.SceneComponent|GetRelativeRotation NewParam)) (.yaw _relativerotation))) "1.000000,1.000000,1.000000") "AdjustIfPossibleButAlwaysSpawn" 0 0))
    (if (and (Utilities|IsValid _returnvalue) (Utilities|IsValid _targetactor))
      (if (Variables|Default|GetIsHoming)
        (bind _asprojectile (Utilities|Casting|CastToProjectile _returnvalue))
        (Variables|/Script/Engine.ProjectileMovementComponent|SetHomingTargetComponent (Variables|/Game/MainGameAssets/Blueprints/Projectile.Projectile_C|GetProjectileMovement _asprojectile) (Variables|/Script/Engine.Actor|GetRootComponent _targetactor))))))