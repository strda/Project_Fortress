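; Wave-based enemy spawner that rides along a track spline via a timeline and registers itself with KeplerGameMode.
; While its wave gate is open, Tick counts down and spawns a random Wolf, Shroom or Golem from the current wave's remaining counts.
; Opening the gate advances the wave and shortens the clamped spawn delay.
; Closing it restores wave and building UI once no enemies remain, showing the win screen after the final wave.
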(event Custom|MoveSpawn
  ;[1 1 1] Spawner mover
  (Components|Timeline|SetPlayRate (Variables|Default|GetCartMover) (/ (Variables|TrackStuffs|GetDuration%28speed%29) 1e+01))
  (bind _alpha (Timeline|CartMover PlayFromStart)
    (:Update
      (Variables|Trackstuffs|SetAlpha _alpha)
      (Transformation|SetActorLocationAndRotation (Spline|GetLocationatDistanceAlongSpline (Variables|/Game/MainGameAssets/Blueprints/Enemies/SpawnerTrack_bp.SpawnerTrack_bp_C|GetSplineTrack (Variables|TrackStuffs|GetTrackRef)) (Math|Float|Lerp 0.0 (Spline|GetSplineLength (Variables|/Game/MainGameAssets/Blueprints/Enemies/SpawnerTrack_bp.SpawnerTrack_bp_C|GetSplineTrack (Variables|TrackStuffs|GetTrackRef))) (Variables|Trackstuffs|GetAlpha)) "World") (Spline|GetRotationatDistanceAlongSpline (Variables|/Game/MainGameAssets/Blueprints/Enemies/SpawnerTrack_bp.SpawnerTrack_bp_C|GetSplineTrack (Variables|TrackStuffs|GetTrackRef)) (Math|Float|Lerp 0.0 (Spline|GetSplineLength (Variables|/Game/MainGameAssets/Blueprints/Enemies/SpawnerTrack_bp.SpawnerTrack_bp_C|GetSplineTrack (Variables|TrackStuffs|GetTrackRef))) (Variables|Trackstuffs|GetAlpha)) "World")))))

(event Custom|OpenWaveGate
  (CallFunction|StartWave)
  (Utilities|FlowControl|Gate true) ; enters at Open
)

(event Custom|CloseWaveGate
  (CallFunction|EndWave)
  (Utilities|FlowControl|Gate true) ; enters at Close
)

(event EventBeginPlay
  (CallFunction|MoveSpawn)
  (bind _askepler_game_mode (Utilities|Casting|CastToKeplerGameMode (Game|GetGameMode)))
  (bind _output_get (Variables|spawningstuffs|SetGamemodeRef _askepler_game_mode))
  (Variables|/Game/MainGameAssets/Blueprints/KeplerGameMode.KeplerGameMode_C|SetEnemySpawner _output_get self)
  (Variables|SpawningStuffs|SetCurrentTime (Variables|SpawningStuffs|GetDelayTime)))

(event EventTick
  (params (DeltaSeconds :type Float%20%28single-precision%29))
  (Utilities|FlowControl|Gate true
    (:Exit
      (bind _isempty (CallFunction|CheckforAllEnemiesSpawned))
      (if (not _isempty)
        (if (> (Variables|SpawningStuffs|GetCurrentTime) 0.0)
          (Variables|SpawningStuffs|SetCurrentTime (- (Variables|SpawningStuffs|GetCurrentTime) DeltaSeconds))
          (else
            (CallFunction|SpawnRandomEnemyType)
            (Variables|SpawningStuffs|SetCurrentTime (Variables|SpawningStuffs|GetDelayTime))))))))

(fn ConstructionScript)

(fn SpawnRandomEnemyType
  (bind _returnvalue (Transformation|GetActorLocation))
  (bind _waves (Variables|Default|GetWaves))
  (bind _gamemoderef (Variables|spawningstuffs|GetGamemodeRef))
  (bind _gamemoderef_2 (Variables|spawningstuffs|GetGamemodeRef))
  (bind _wavenum (Variables|/Game/MainGameAssets/Blueprints/KeplerGameMode.KeplerGameMode_C|GetWaveNum _gamemoderef))
  (bind _output (Utilities|Array|Get(acopy) _waves _wavenum))
  (bind _enemytypename (CallFunction|GetRandomEnemyTypeName))
  (switch name _enemytypename
    (:Wolf
      (AI|SpawnAIFromClass "/Game/MainGameAssets/Blueprints/Enemies/WolfEnemy_BP.WolfEnemy_BP_C" 0 _returnvalue "0, 0, 0" false 0)
      (Math|Integer|DecrementInt (.wolfcount _output)
        (:%20%20
          _)))
    (:Shroom
      (AI|SpawnAIFromClass "/Game/MainGameAssets/Blueprints/Enemies/MushroomEnemy_BP.MushroomEnemy_BP_C" 0 _returnvalue "0, 0, 0" false 0)
      (Math|Integer|DecrementInt (.shroomcount _output)
        (:%20%20
          _)))
    (:Golem
      (AI|SpawnAIFromClass "/Game/MainGameAssets/Blueprints/Enemies/GolemEnemy_BP.GolemEnemy_BP_C" 0 _returnvalue "0, 0, 0" false 0)
      (Math|Integer|DecrementInt (.golemcount _output)
        (:%20%20
          _))))
  (Variables|SpawningStuffs|SetEnemiesToSpawn (- (Variables|SpawningStuffs|GetEnemiesToSpawn) 1))
  (Variables|/Game/MainGameAssets/Blueprints/KeplerGameMode.KeplerGameMode_C|SetEnemiesAlive _gamemoderef_2 (+ (Variables|/Game/MainGameAssets/Blueprints/KeplerGameMode.KeplerGameMode_C|GetEnemiesAlive _gamemoderef_2) 1)))

(fn StartWave
  (bind _gamemoderef (Variables|spawningstuffs|GetGamemodeRef))
  (bind _output_get (Variables|/Game/MainGameAssets/Blueprints/KeplerGameMode.KeplerGameMode_C|SetWaveNum _gamemoderef (Variables|/Game/MainGameAssets/Blueprints/KeplerGameMode.KeplerGameMode_C|GetWaveNum _gamemoderef)))
  (Math|Integer|IncrementInt _output_get
    (:%20%20
      (Variables|SpawningStuffs|SetDelayTime (Math|Float|Clamp(Float) (- (Variables|SpawningStuffs|GetDelayTime) 0.2) 0.8 1.6)))))

(fn EndWave
  (bind _gamemoderef (Variables|spawningstuffs|GetGamemodeRef))
  (bind _asrtsplayer_controller_bp (Utilities|Casting|CastToRTSPlayerController_BP (Game|GetPlayerController 0)))
  (if (== (Variables|/Game/MainGameAssets/Blueprints/KeplerGameMode.KeplerGameMode_C|GetEnemiesAlive _gamemoderef) 0)
    (Widget|SetVisibility (Variables|/Game/MainGameAssets/UI/HUD.HUD_C|GetWaveButton (Variables|/Game/MainGameAssets/Blueprints/RTSPlayerController_BP.RTSPlayerController_BP_C|GetHUD_REF _asrtsplayer_controller_bp)) "Visible")
    (Default|LockBuildingMenuUI (Variables|/Game/MainGameAssets/Blueprints/RTSPlayerController_BP.RTSPlayerController_BP_C|GetHUD_REF _asrtsplayer_controller_bp) false)
    (if (>= (Variables|/Game/MainGameAssets/Blueprints/KeplerGameMode.KeplerGameMode_C|GetWaveNum _gamemoderef) (- (Utilities|Array|Length (Variables|Default|GetWaves)) 1))
      (Widget|SetVisibility (Variables|/Game/MainGameAssets/Blueprints/RTSPlayerController_BP.RTSPlayerController_BP_C|GetHUD_REF _asrtsplayer_controller_bp) "Collapsed")
      (bind _returnvalue (UserInterface|CreateWidget "/Game/MainGameAssets/UI/WinScreen.WinScreen_C"))
      (UserInterface|Viewport|AddtoViewport _returnvalue 0))))

(fn CheckforAllEnemiesSpawned
  (bind _waves (Variables|Default|GetWaves))
  (bind _gamemoderef (Variables|spawningstuffs|GetGamemodeRef))
  (bind _wavenum (Variables|/Game/MainGameAssets/Blueprints/KeplerGameMode.KeplerGameMode_C|GetWaveNum _gamemoderef))
  (bind _output (Utilities|Array|Get(acopy) _waves _wavenum))
  (if (== (+ (.wolfcount _output) (.shroomcount _output) (.golemcount _output)) 0)
    (return true)
    (else
      (return false))))

(fn GetRandomEnemyTypeName
  (bind _availablespawningtypes (Variables|Default|GetAvailableSpawningTypes))
  (bind _waves (Variables|Default|GetWaves))
  (bind _gamemoderef (Variables|spawningstuffs|GetGamemodeRef))
  (bind _wavenum (Variables|/Game/MainGameAssets/Blueprints/KeplerGameMode.KeplerGameMode_C|GetWaveNum _gamemoderef))
  (bind _output (Utilities|Array|Get(acopy) _waves _wavenum))
  (Utilities|FlowControl|Sequence
    (:then_0
      (if (> (.wolfcount _output) 0)
        (if (== (Utilities|Array|FindItem _availablespawningtypes "Wolf") -1)
          (Utilities|Array|Add _availablespawningtypes "Wolf"))
        (else
          (Utilities|Array|RemoveItem _availablespawningtypes "Wolf"))))
    (:then_1
      (if (> (.shroomcount _output) 0)
        (if (== (Utilities|Array|FindItem _availablespawningtypes "Shroom") -1)
          (Utilities|Array|Add _availablespawningtypes "Shroom"))
        (else
          (Utilities|Array|RemoveItem _availablespawningtypes "Shroom"))))
    (:then_2
      (if (> (.golemcount _output) 0)
        (if (== (Utilities|Array|FindItem _availablespawningtypes "Golem") -1)
          (Utilities|Array|Add _availablespawningtypes "Golem"))
        (else
          (Utilities|Array|RemoveItem _availablespawningtypes "Golem"))))
    (:then_3
      (return (Utilities|Array|Get(acopy) _availablespawningtypes (Math|Random|RandomInteger (Utilities|Array|Length _availablespawningtypes)))))))