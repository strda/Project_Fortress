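; Standard enemy character that advances on the town hall and pays out gold when killed.
; It takes its target from KeplerGameMode and reissues AIMoveTo every Tick until the Detect component overlaps a TownHall_BP, then halts its movement.
; Damage lowers Health and refreshes the health bar widget, and at zero the enemy adds its Value to the game mode's Gold and destroys itself.
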(event OnComponentBeginOverlap(Detect)
  (params (OverlappedComponent :type Primitive%20Component%20Object%20Reference) (OtherActor :type Actor%20Object%20Reference) (OtherComp :type Primitive%20Component%20Object%20Reference) (OtherBodyIndex :type Integer) (bFromSweep :type Boolean) (SweepResult :type Hit%20Result%20Structure%20%28by%20ref%29))
  (bind _astown_hall_bp (Utilities|Casting|CastToTownHall_BP OtherActor))
  (Utilities|IsValid _astown_hall_bp
    (:Is%20Valid
      (Variables|Default|SetTHDetected true))))

(event EventBeginPlay
  (bind _askepler_game_mode (Utilities|Casting|CastToKeplerGameMode (Game|GetGameMode)))
  (Variables|Default|SetTarget (Variables|/Game/MainGameAssets/Blueprints/KeplerGameMode.KeplerGameMode_C|GetTownHallBuilding _askepler_game_mode))
  (CallFunction|UpdateHealthBar))

(event Collision|EventActorBeginOverlap
  (params (OtherActor :type Actor%20Object%20Reference)))

(event EventTick
  (params (DeltaSeconds :type Float%20%28single-precision%29))
  (if (Variables|Default|GetTHDetected)
    (Class|NavMovementComponent|StopActiveMovement (Variables|Character|GetCharacterMovement))
    (else
      (AI|AIMoveTo self "0, 0, 0" (Variables|Default|GetTarget) 5.0 false))))

(event Game|Damage|EventAnyDamage
  (params (Damage :type Float%20%28single-precision%29) (DamageType :type Damage%20Type%20Object%20Reference) (InstigatedBy :type Controller%20Object%20Reference) (DamageCauser :type Actor%20Object%20Reference))
  (Variables|Default|SetHealth (- (Variables|Default|GetHealth) Damage))
  (CallFunction|UpdateHealthBar)
  (if (<= (Variables|Default|GetHealth) 0.0)
    (bind _askepler_game_mode (Utilities|Casting|CastToKeplerGameMode (Game|GetGameMode)))
    (Variables|/Game/MainGameAssets/Blueprints/KeplerGameMode.KeplerGameMode_C|SetGold _askepler_game_mode (+ (Variables|/Game/MainGameAssets/Blueprints/KeplerGameMode.KeplerGameMode_C|GetGold _askepler_game_mode) (Math|Float|Truncate (Variables|Default|GetValue))))
    (Actor|DestroyActor)))

(fn ConstructionScript)

(fn UpdateHealthBar
  (bind _ashealth_bar (Utilities|Casting|CastToHealthBar (UserInterface|GetUserWidgetObject (Variables|Default|GetWidget))))
  (Variables|/Game/MainGameAssets/UI/HealthBar.HealthBar_C|SetHealth _ashealth_bar (/ (Variables|Default|GetHealth) (Variables|Default|GetMaxHealth)))
  (return))