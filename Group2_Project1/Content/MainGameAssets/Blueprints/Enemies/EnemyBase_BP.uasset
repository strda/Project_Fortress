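; Base enemy character that marches on the town hall taken from KeplerGameMode and damages it.
; Tick drives AI movement toward the hall until a Detect overlap stops it and starts timed attacks.
; Incoming damage updates a health bar widget.
; On death it grants scrap, decrements the alive count, tells the spawner to close the wave gate when none remain, and destroys itself.
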(event OnComponentBeginOverlap(Detect)
  (params (OverlappedComponent :type Primitive%20Component%20Object%20Reference) (OtherActor :type Actor%20Object%20Reference) (OtherComp :type Primitive%20Component%20Object%20Reference) (OtherBodyIndex :type Integer) (bFromSweep :type Boolean) (SweepResult :type Hit%20Result%20Structure%20%28by%20ref%29))
  (bind _astown_hall_bp (Utilities|Casting|CastToTownHall_BP OtherActor))
  (Utilities|IsValid _astown_hall_bp
    (:Is%20Valid
      (Variables|Default|SetTHDetected true))))

(event EventBeginPlay
  (Variables|Default|SetCurrentHealth (Variables|Default|GetMaxHealth))
  (Variables|/Script/Engine.CharacterMovementComponent|SetMaxWalkSpeed (Variables|Character|GetCharacterMovement) (Variables|Default|GetMoveSpeed))
  (bind _askepler_game_mode (Utilities|Casting|CastToKeplerGameMode (Game|GetGameMode)))
  (Variables|Default|SetTarget (Variables|/Game/MainGameAssets/Blueprints/KeplerGameMode.KeplerGameMode_C|GetTownHallBuilding _askepler_game_mode))
  (CallFunction|UpdateHealthBar)
  (Variables|Default|SetCurrentAttackTime (Variables|Default|GetDelayAttackTime)))

(event EventTick
  (params (DeltaSeconds :type Float%20%28single-precision%29))
  (Utilities|IsValid (Variables|Default|GetTarget)
    (:Is%20Valid
      (if (Variables|Default|GetTHDetected)
        (Class|NavMovementComponent|StopActiveMovement (Variables|Character|GetCharacterMovement))
        (Variables|Default|SetCurrentAttackTime (- (Variables|Default|GetCurrentAttackTime) DeltaSeconds))
        (if (<= (Variables|Default|GetCurrentAttackTime) 0.0)
          (Default|ChangeHealth (Variables|Default|GetTarget) (* (Variables|Default|GetDamage) -1))
          (Variables|Default|SetCurrentAttackTime (Variables|Default|GetDelayAttackTime)))
        (else
          (AI|AIMoveTo self "0, 0, 0" (Variables|Default|GetTarget) 5.0 false))))))

(event Game|Damage|EventAnyDamage
  (params (Damage :type Float%20%28single-precision%29) (DamageType :type Damage%20Type%20Object%20Reference) (InstigatedBy :type Controller%20Object%20Reference) (DamageCauser :type Actor%20Object%20Reference))
  (Variables|Default|SetCurrentHealth (- (Variables|Default|GetCurrentHealth) Damage))
  (CallFunction|UpdateHealthBar)
  (if (<= (Variables|Default|GetCurrentHealth) 0.0)
    (CallFunction|KillEnemy)))

(fn ConstructionScript)

(fn UpdateHealthBar
  (bind _ashealth_bar (Utilities|Casting|CastToHealthBar (UserInterface|GetUserWidgetObject (Variables|Default|GetWidget))))
  (Variables|/Game/MainGameAssets/UI/HealthBar.HealthBar_C|SetHealth _ashealth_bar (/ (Variables|Default|GetCurrentHealth) (Variables|Default|GetMaxHealth)))
  (return))

(fn KillEnemy
  (bind _askepler_game_mode (Utilities|Casting|CastToKeplerGameMode (Game|GetGameMode)))
  (Default|ChangeScrapCount _askepler_game_mode (Variables|Default|GetEnemyScrap))
  (bind _output_get (Variables|/Game/MainGameAssets/Blueprints/KeplerGameMode.KeplerGameMode_C|SetEnemiesAlive _askepler_game_mode (- (Variables|/Game/MainGameAssets/Blueprints/KeplerGameMode.KeplerGameMode_C|GetEnemiesAlive _askepler_game_mode) 1)))
  (if (> _output_get 0)
    (Actor|DestroyActor)
    (else
      (Default|CloseWaveGate (Variables|/Game/MainGameAssets/Blueprints/KeplerGameMode.KeplerGameMode_C|GetEnemySpawner _askepler_game_mode))
      (Actor|DestroyActor))))