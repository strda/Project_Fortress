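; RTS camera actor that becomes player 0's view target on BeginPlay and edge-scrolls with the mouse.
; Each Tick, horizontal and vertical functions offset the root when the cursor enters the outer 5% viewport bands.
; Speed ramps toward the screen edge, except on the right, where the reversed normalize range makes it fall to zero.
; Movement is per frame, with no delta-time scaling or bounds.
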(event EventBeginPlay
  (Game|Player|SetViewTargetwithBlend (Game|GetPlayerController 0) self 0.0 "VTBlend_Linear" 0.0 false))

(event EventTick
  (params (DeltaSeconds :type Float%20%28single-precision%29))
  (CallFunction|MoveCameraHorizontal)
  (CallFunction|MoveCameraVertical))

(fn ConstructionScript)

(fn MoveCameraHorizontal
  (bind _returnvalue (Viewport|GetViewportSize))
  (bind _defaultsceneroot (Variables|Default|GetDefaultSceneRoot))
  (bind _returnvalue_2 (Class|WidgetLayoutLibrary|GetMousePositiononViewport))
  (if (>= (/ (.x _returnvalue_2) (.x _returnvalue)) 0.95)
    (Transformation|AddRelativeLocation _defaultsceneroot (* (Math|Float|Clamp(Float) (Math|Float|NormalizetoRange (.x _returnvalue_2) (.x _returnvalue) (* (.x _returnvalue) 0.95))) "-100.000000,0.000000,0.000000") false false)
    (elif (<= (/ (.x _returnvalue_2) (.x _returnvalue)) 0.05)
      (Transformation|AddRelativeLocation _defaultsceneroot (* (- 1.0 (Math|Float|Clamp(Float) (Math|Float|NormalizetoRange (.x _returnvalue_2) 0.0 (* (.x _returnvalue) 0.05)))) "100.000000,0.000000,0.000000") false false))))

(fn MoveCameraVertical
  (bind _returnvalue (Viewport|GetViewportSize))
  (bind _defaultsceneroot (Variables|Default|GetDefaultSceneRoot))
  (bind _returnvalue_2 (Class|WidgetLayoutLibrary|GetMousePositiononViewport))
  (if (>= (/ (.y _returnvalue_2) (.y _returnvalue)) 0.95)
    (Transformation|AddRelativeLocation _defaultsceneroot (* (Math|Float|Clamp(Float) (Math|Float|NormalizetoRange (.y _returnvalue_2) (* (.y _returnvalue) 0.95) (.y _returnvalue))) "0.000000,-100.000000,0.000000") false false)
    (elif (<= (/ (.y _returnvalue_2) (.y _returnvalue)) 0.05)
      (Transformation|AddRelativeLocation _defaultsceneroot (* (- 1.0 (Math|Float|Clamp(Float) (Math|Float|NormalizetoRange (.y _returnvalue_2) 0.0 (* (.y _returnvalue) 0.05)))) "0.000000,100.000000,0.000000") false false))))