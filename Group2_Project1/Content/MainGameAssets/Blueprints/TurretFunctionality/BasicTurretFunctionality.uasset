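; Shared turret targeting logic that finds enemies within range and turns the turret's rotating part toward one.
; RotateToObject sphere-overlaps EnemyBase_BP pawns around Parent and stores the nearest as TargetActor.
; GolemEnemyFixed is passed over when other enemies are present, though a golem last in the list triggers a rescan that can select it.
; ObjectRotating gets an interpolated yaw-only look-at with a 90-degree offset, and TargetFound reports the result.
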(event EventBeginPlay
  (|CallParentFunction) ; This node is disabled and will not be called.\nDrag off pins to build functionality.
)

(event EventTick
  (params (DeltaSeconds :type Float%20%28single-precision%29))
  (|CallParentFunction DeltaSeconds) ; This node is disabled and will not be called.\nDrag off pins to build functionality.
)

(fn RotatetoObject
  (bind _parent (Variables|Default|GetParent))
  (Variables|Default|SetDistanceToTarget (Variables|Default|GetRange))
  (bind (_outactors _returnvalue) (Collision|SphereOverlapActors (Transformation|GetActorLocation _parent) (Variables|Default|GetRange) (Utilities|Array|MakeArray "ObjectTypeQuery3") "/Game/MainGameAssets/Blueprints/Enemies/EnemyBase_BP.EnemyBase_BP_C")) ; Enemy class will be put in the actor class filter once it is implemented into the game
  (if _returnvalue
    (for (_array_element _array_index) _outactors
      (if (< (Transformation|GetDistanceTo _parent _array_element) (Variables|Default|GetDistanceToTarget))
        (if (and (> (Utilities|Array|Length _outactors) 1) (== (Utilities|GetClass _array_element) "/Game/MainGameAssets/Blueprints/Enemies/golem/GolemEnemyFixed.GolemEnemyFixed_C"))
          (if (== _array_index (- (Utilities|Array|Length _outactors) 1))
            (for _array_element_2 _outactors
              (if (< (Transformation|GetDistanceTo _parent _array_element_2) (Variables|Default|GetDistanceToTarget))
                (Variables|Default|SetDistanceToTarget (Transformation|GetDistanceTo _parent _array_element_2))
                (Variables|Default|SetTargetActor _array_element_2))))
          (else
            (Variables|Default|SetDistanceToTarget (Transformation|GetDistanceTo _parent _array_element))
            (Variables|Default|SetTargetActor _array_element)))))
    (if (Utilities|IsValid (Variables|Default|GetTargetActor))
      (Transformation|SetRelativeRotation (Variables|Default|GetObjectRotating) (Math|Interpolation|RInterpTo (Transformation|GetActorRotation _parent) (Math|Rotator|MakeRotator 0.0 0.0 (- (.Yaw (Math|Rotator|BreakRotator (Math|Rotator|FindLookatRotation (Transformation|GetActorLocation _parent) (Transformation|GetActorLocation (Variables|Default|GetTargetActor))))) 9e+01)) 1.0 (Variables|Default|GetInterpSpeed)) false false)
      (Variables|Default|SetTargetFound true))
    (else
      (Variables|Default|SetTargetFound false))))