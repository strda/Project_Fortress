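; Ghost placement preview for the building system, showing the selected building's mesh at the grid-snapped cursor position while flagging the game mode's build mode as active.
; ConstructBuilding briefly spawns the building to read its mesh and proxy, then destroys it.
; A gated Tick moves the ghost and swaps to an error material when it overlaps any actor.
; GetConstructionStruct packages the classes, mesh and transform for construction.
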(event Custom|OnSpawn
  (params (DisplayMesh :type Static%20Mesh%20Object%20Reference) (BuildingClass :type Building%20BP%20Class%20Reference) (ConstructionProxy :type Construction%20Proxy%20BP%20Class%20Reference))
  ;[1 1 1] On Spawn Ghost
  (if (not (Variables|Default|GetIsActive))
    (Variables|Default|SetBuildingClass BuildingClass)
    (Variables|Default|SetBuildingProxy ConstructionProxy)
    (Variables|Default|SetDisplayMesh DisplayMesh)
    (Variables|Default|SetIsActive true)
    (Variables|/Game/MainGameAssets/Blueprints/KeplerGameMode.KeplerGameMode_C|SetBuildModeActive (Variables|/Game/MainGameAssets/Blueprints/RTSPlayerController_BP.RTSPlayerController_BP_C|GetGameModeRef (Variables|References|GetControllerRef)) true)
    (Components|StaticMesh|SetStaticMesh (Variables|Default|GetGhostBuildingMesh) (Variables|Default|GetDisplayMesh))
    (CallFunction|OpenTickGate)
    (CallFunction|SetStatusMaterial (not (Variables|Default|GetIsOverlapping)))))

(event Custom|KillGhost
  ;[1 1 1] On Kill Ghost
  (Variables|Default|SetBuildingClass 0)
  (Variables|Default|SetBuildingProxy 0)
  (CallFunction|CloseTickGate)
  (Variables|Default|SetDisplayMesh 0)
  (Variables|Default|SetIsActive false)
  (Variables|/Game/MainGameAssets/Blueprints/KeplerGameMode.KeplerGameMode_C|SetBuildModeActive (Variables|/Game/MainGameAssets/Blueprints/RTSPlayerController_BP.RTSPlayerController_BP_C|GetGameModeRef (Variables|References|GetControllerRef)) false)
  (Components|StaticMesh|SetStaticMesh (Variables|Default|GetGhostBuildingMesh) (Variables|Default|GetDisplayMesh)) ; Setting Ghost Mesh to null display mesh
)

(event Custom|OpenTickGate
  ;[1 1 1] Tick
  (Utilities|FlowControl|Gate true) ; enters at Open
)

(event Custom|CloseTickGate
  ;[1 1 1] Tick
  (Utilities|FlowControl|Gate true) ; enters at Close
)

(event Custom|SetStatusMaterial
  (params (IsError :type Boolean))
  (bind _ghostbuildingmesh (Variables|Default|GetGhostBuildingMesh))
  (if (not (== IsError (Variables|Default|GetIsOverlapping)))
    (bind _output_get (Variables|Default|SetIsOverlapping IsError))
    (if _output_get
      (Rendering|Material|SetMaterial _ghostbuildingmesh 0 "/Game/MainGameAssets/Materials/BuildingMats/GhostBuildingError.GhostBuildingError")
      (else
        (Rendering|Material|SetMaterial _ghostbuildingmesh 0 "/Game/MainGameAssets/Materials/BuildingMats/GhostBuildingInstance.GhostBuildingInstance")))))

(event EventTick
  (params (DeltaSeconds :type Float%20%28single-precision%29))
  ;[1 1 1] Tick
  (Utilities|FlowControl|Gate true
    (:Exit
      (Transformation|SetActorLocation self (CallFunction|SetGridSnapVector) false false)
      (if (CallFunction|CheckOverlap)
        (CallFunction|SetStatusMaterial true)
        (else
          (CallFunction|SetStatusMaterial false))))))

(event EventConstructBuilding
  (params (Building :type Building%20BP%20Class%20Reference))
  (bind _returnvalue (Game|SpawnActorfromClass Building (Math|Transform|MakeTransform "0, 0, 0") "Undefined" 0 (Variables|References|GetControllerRef) 0))
  (Utilities|FlowControl|Sequence
    (:then_0
      (bind _asbuilding_bp (Utilities|Casting|CastToBuilding_BPClass Building))
      (CallFunction|KillGhost)
      (CallFunction|OnSpawn (Variables|/Game/MainGameAssets/Blueprints/BuildingSystemBluePrints/BuildingClasses/Building_BP.Building_BP_C|GetDisplayMesh _returnvalue) _asbuilding_bp (Variables|/Game/MainGameAssets/Blueprints/BuildingSystemBluePrints/BuildingClasses/Building_BP.Building_BP_C|GetConstructionProxy _returnvalue)))
    (:then_1
      (Actor|DestroyActor _returnvalue) ; Could Set Building BP to hidden by default. When spawning could set visibility to true\ninstead of destroying the actor
    )))

(fn ConstructionScript)

(fn SetGridSnapVector
  (bind _cursorworldposition (Variables|Default|GetCursorWorldPosition))
  (bind _gridsize (Variables|Default|GetGridSize))
  (return (Math|Vector|MakeVector (CallFunction|SnaptoGrid (.x _cursorworldposition) _gridsize) (CallFunction|SnaptoGrid (.y _cursorworldposition) _gridsize) (CallFunction|SnaptoGrid (.z _cursorworldposition) _gridsize))))

(fn SetCursorPosition
  (params (CursorPosition :type Vector))
  (Variables|Default|SetCursorWorldPosition CursorPosition)
  (return))

(fn GetConstructionStruct
  (return (Utilities|Struct|MakeConstructionStruct (Variables|Default|GetBuildingClass) (Variables|Default|GetBuildingProxy) (Math|Transform|MakeTransform (Transformation|GetActorLocation) (Transformation|GetActorRotation) (Transformation|GetActorScale3D)) (Variables|Default|GetDisplayMesh))))

(fn CheckOverlap
  (return (> (Utilities|Array|Length (Collision|GetOverlappingActors "/Script/Engine.Actor" :!class /Script/Engine.Actor)) 0)))