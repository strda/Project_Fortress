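; Town hall building for the base-building and wave game, extending a parent building class.
; When it begins play enabled, it registers with KeplerGameMode, refreshes the HUD's building menu and reveals the wave button.
; Its upgrade override steps through tiers: one unlocks the mortar ability and sets up the next upgrade's description and cost, another raises max health and fully heals it.
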(event EventBeginPlay
  (bind _controllerref (Variables|Default|GetControllerRef))
  (bind _hud_ref (Variables|/Game/MainGameAssets/Blueprints/RTSPlayerController_BP.RTSPlayerController_BP_C|GetHUD_REF _controllerref))
  (|CallParentFunction)
  (if (Variables|Default|GetBuildingEnabled)
    (bind _askepler_game_mode (Utilities|Casting|CastToKeplerGameMode (Game|GetGameMode)))
    (Variables|/Game/MainGameAssets/Blueprints/KeplerGameMode.KeplerGameMode_C|SetTownHallBuilding _askepler_game_mode self)
    (Variables|/Game/MainGameAssets/UI/HUD.HUD_C|SethasPlacedTownHall _hud_ref true)
    (Default|UpdateBuildingMenuButtons _hud_ref)
    (Widget|SetVisibility (Variables|/Game/MainGameAssets/UI/HUD.HUD_C|GetWaveButton _hud_ref) "Visible")))

(fn ConstructionScript
  (|CallParentFunction))

(fn UpgradeBuilding
  (bind _controllerref (Variables|Default|GetControllerRef))
  (bind _hud_ref (Variables|/Game/MainGameAssets/Blueprints/RTSPlayerController_BP.RTSPlayerController_BP_C|GetHUD_REF _controllerref))
  (|CallParentFunction)
  (bind _result (Math|Integer|IncrementInt (Variables|Default|GetCurrUpgradeNum))
    (:%20%20
      (bind _output_get (Variables|Default|SetCurrUpgradeNum _result))
      (switch int _output_get
        (:0
          (Default|UnlockMortarAbilityUI _hud_ref)
          (Variables|/Game/MainGameAssets/Blueprints/KeplerGameMode.KeplerGameMode_C|SetMortarUnlocked (Variables|/Game/MainGameAssets/Blueprints/RTSPlayerController_BP.RTSPlayerController_BP_C|GetGameModeRef _controllerref) true)
          (Variables|/Game/MainGameAssets/Blueprints/RTSPlayerController_BP.RTSPlayerController_BP_C|SetCanUseMortar _controllerref true)
          (Variables|Default|SetUpgradeDesc "Increases Max Health and Fully Heals Reactor")
          (Variables|Default|SetUpgradeCost (+ (Variables|Default|GetUpgradeCost) 10)))
        (:1
          (bind _output_get_2 (Variables|Default|SetMaxHealth (+ (Variables|Default|GetMaxHealth) 5)))
          (bind _output_get_3 (Variables|Default|SetCurrentHealth _output_get_2))
          (Default|UpdateBuildingSelectionHealthbar _hud_ref _output_get_3 _output_get_2))))))