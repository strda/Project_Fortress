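; Turret building Blueprint, a child building class with health, selection UI and tiered upgrades.
; On begin play it fills health and binds to the controller's HUD request, updating the selection UI when this turret is picked.
; Health changes are clamped, destroy the actor at zero or below, and refresh healthbars.
; Upgrades step through TurretUpgrades by swapping the child actor class and raising the cost.
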(event Custom|DisplayTurretHUD
  (params (Actor :type Actor%20Object%20Reference))
  (bind _self self)
  (if (== Actor _self)
    (Variables|Default|SetBuildingSelected true)
    (Default|UpdateBuildingSelectionUI (Variables|/Game/MainGameAssets/Blueprints/RTSPlayerController_BP.RTSPlayerController_BP_C|GetHUD_REF (Variables|Default|GetControllerRef)) _self)))

(event EventBeginPlay
  (Variables|Default|SetCurrentHealth (Variables|Default|GetMaxHealth))
  (EventDispatchers|BindEventtoHUDRequest (Variables|Default|GetControllerRef) (EventDispatchers|CreateEvent :!event Custom|DisplayTurretHUD))
  (CallFunction|UpdateBuildingHealthbar)
  (Variables|Default|SetMaxUpgradeNum (Utilities|Array|Length (Variables|Default|GetturretUpgrades))))

(fn ConstructionScript
  (|CallParentFunction))

(fn ChangeHealth
  (params (healthValue :type Integer))
  (bind _maxhealth (Variables|Default|GetMaxHealth))
  (bind _output_get (Variables|Default|SetCurrentHealth (Math|Integer|Clamp(Integer) (+ healthValue (Variables|Default|GetCurrentHealth)) -1 _maxhealth)))
  (if (<= _output_get 0) ; Check for Building Destruction
    (Actor|DestroyActor)
    (else
      (CallFunction|UpdateBuildingHealthbar)
      (if (Variables|Default|GetBuildingSelected)
        (Default|UpdateBuildingSelectionHealthbar (Variables|/Game/MainGameAssets/Blueprints/RTSPlayerController_BP.RTSPlayerController_BP_C|GetHUD_REF (Variables|Default|GetControllerRef)) _output_get _maxhealth)))))

(fn UpgradeBuilding
  (bind _turretupgrades (Variables|Default|GetturretUpgrades))
  (bind _currupgradenum (Variables|Default|GetCurrUpgradeNum))
  (if (!= _currupgradenum (- (Utilities|Array|Length _turretupgrades) 1))
    (bind _result (Math|Integer|IncrementInt _currupgradenum)
      (:%20%20
        (ChildActorComponent|SetChildActorClass (Variables|Default|GetupgradeChildActor) (Utilities|Array|Get(acopy) _turretupgrades _result))
        (Variables|Default|SetUpgradeCost (+ (Variables|Default|GetUpgradeCost) 5))))))