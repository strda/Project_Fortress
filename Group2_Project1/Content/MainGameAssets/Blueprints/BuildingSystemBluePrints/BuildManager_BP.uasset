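; BuildManager_BP places buildings in the game, paying for them with the scrap count held by KeplerGameMode.
; It caches the game mode on BeginPlay.
; ConstructBuilding takes a struct of class, transform and cost, checking affordability and whether the RTS player controller's ghost building is in a placement zone.
; On success it spawns the enabled building regardless of collision, passing it the controller, then deducts the cost.
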(event EventBeginPlay
  (bind _askepler_game_mode (Utilities|Casting|CastToKeplerGameMode (Game|GetGameMode)))
  (Variables|Default|SetKeplerGamemode _askepler_game_mode))

(fn ConstructionScript)

(fn ConstructBuilding
  (params (Construction%20Struct :type Construction%20Struct%20Structure))
  (bind (_buildingclass _transform _displaymesh _buildingcost) (Utilities|Struct|BreakConstructionStruct Construction%20Struct))
  (bind _keplergamemode (Variables|Default|GetKeplerGamemode))
  (if (<= _buildingcost (Variables|/Game/MainGameAssets/Blueprints/KeplerGameMode.KeplerGameMode_C|GetScrapCount _keplergamemode))
    (bind _asrtsplayer_controller_bp (Utilities|Casting|CastToRTSPlayerController_BP (Game|GetPlayerController 0)))
    (if (Variables|/Game/MainGameAssets/Blueprints/BuildingSystemBluePrints/GhostBuilding_BP.GhostBuilding_BP_C|GetInPlacementZone (Variables|/Game/MainGameAssets/Blueprints/RTSPlayerController_BP.RTSPlayerController_BP_C|GetGhostBuildingRef _asrtsplayer_controller_bp))
      (Game|SpawnActorfromClass _buildingclass _transform "AlwaysSpawn" 0 _asrtsplayer_controller_bp true 0)
      (Variables|/Game/MainGameAssets/Blueprints/KeplerGameMode.KeplerGameMode_C|SetScrapCount _keplergamemode (- (Variables|/Game/MainGameAssets/Blueprints/KeplerGameMode.KeplerGameMode_C|GetScrapCount _keplergamemode) _buildingcost)))))